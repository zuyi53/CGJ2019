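; A rotating target actor that randomly wants a heart or cash and awards points when the matching actor touches it.
; The construction script randomly picks the mesh and Type, and a Timeline started at BeginPlay drives its yaw.
; On box overlap it searches all actors of the matching class (Heart or Cash_b) for the other actor.
; A match prints a message, destroys this actor and adds type-specific points to MyGameState; each non-match prints a puzzled message.
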(event OnComponentBeginOverlap(Box)
  (params (OverlappedComponent :type Primitive%20Component%20Object%20Reference) (OtherActor :type Actor%20Object%20Reference) (OtherComp :type Primitive%20Component%20Object%20Reference) (OtherBodyIndex :type Integer) (bFromSweep :type Boolean) (SweepResult :type Hit%20Result%20Structure%20%28by%20ref%29))
  (bind _returnvalue (Game|GetGameState))
  (switch int (Variables|Default|Gettype)
    (:0
      (bind _outactors (Actor|GetAllActorsOfClass "/Game/FirstPersonBP/Blueprints/heart.heart_C"))
      (for _array_element _outactors
        (if (== _array_element OtherActor)
          (Development|PrintString "谢谢")
          (Actor|DestroyActor)
          (bind _asmy_game_state (Utilities|Casting|CastToMyGameState _returnvalue))
          (Variables|/Game/Blueprints/MyGameState.MyGameState_C|Setpoint _asmy_game_state (+ (Variables|/Game/Blueprints/MyGameState.MyGameState_C|Getpoint _asmy_game_state) 100))
          (else
            (Development|PrintString "这是什么？")))))
    (:1
      (bind _outactors_2 (Actor|GetAllActorsOfClass "/Game/FirstPersonBP/Blueprints/cash_b.cash_b_C"))
      (bind _array_element_2 (Utilities|Array|ForEachLoopwithBreak _outactors_2)
        (:LoopBody
          (if (== _array_element_2 OtherActor)
            (Development|PrintString "我们有钱啦")
            (Actor|DestroyActor)
            (bind _asmy_game_state_2 (Utilities|Casting|CastToMyGameState _returnvalue))
            (Variables|/Game/Blueprints/MyGameState.MyGameState_C|Setpoint _asmy_game_state_2 (+ (Variables|/Game/Blueprints/MyGameState.MyGameState_C|Getpoint _asmy_game_state_2) 50))
            (else
              (Development|PrintString "这是什么？"))))))))

(event EventBeginPlay
  (bind _newtrack_0 (Timeline|Timeline_0 Play)
    (:Update
      (Transformation|SetWorldRotation (Variables|Default|GetStaticMesh) (Math|Rotator|MakeRotator 0.0 0.0 _newtrack_0) false false))))

(event Collision|EventActorBeginOverlap
  (params (OtherActor :type Actor%20Object%20Reference)))

(event EventTick
  (params (DeltaSeconds :type Float%20%28single-precision%29)))

(fn ConstructionScript
  (bind _staticmesh (Variables|Default|GetStaticMesh))
  (switch int (Math|Random|RandomInteger 2)
    (:0
      (Components|StaticMesh|SetStaticMesh _staticmesh "/Game/heart.heart")
      (Variables|Default|Settype 0))
    (:1
      (Components|StaticMesh|SetStaticMesh _staticmesh "/Game/cash.cash")
      (Variables|Default|Settype 1))))